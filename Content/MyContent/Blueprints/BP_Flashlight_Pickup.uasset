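; BP_Flashlight_Pickup is a world pickup that gives the first-person player a flashlight.
; On BeginPlay it casts player character 0 to BP_FirstPersonCharacter and caches the reference.
; When that character overlaps the Collision component, it sets the character's HasFlashlight flag, plays a collect sound at its location and destroys itself.
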(event `self.ReceiveBeginPlay`
  ; Setup
  (bind _asbp_first_person_character (cast `/Game/StarterContent/FirstPerson/Blueprints/BP_FirstPersonCharacter` (`GameplayStatics.GetPlayerCharacter` 0)))
  (set `self.BP_FIrstPersonCharacter` _asbp_first_person_character))

(event `self.Collision.OnComponentBeginOverlap`
  (params (OverlappedComponent :type "PrimitiveComponent Object Reference") (OtherActor :type "Actor Object Reference") (OtherComp :type "PrimitiveComponent Object Reference") (OtherBodyIndex :type Integer) (bFromSweep :type Boolean) (SweepResult :type "HitResult Structure (by ref)"))
  (bind _bp_firstpersoncharacter (`self.BP_FIrstPersonCharacter`))
  ; Collect Flashlight
  (if (== OtherActor _bp_firstpersoncharacter)
    (set `/Game/StarterContent/FirstPerson/Blueprints/BP_FirstPersonCharacter.HasFlashlight` true _bp_firstpersoncharacter)
    (`GameplayStatics.PlaySoundAtLocation` "/Game/MyContent/Audio/MP3_Key_Collect.MP3_Key_Collect" (`self.K2_GetActorLocation`) (struct) 1.0 1.0 0.0 null null null null)
    (`self.K2_DestroyActor`)))

(fn `UserConstructionScript`)