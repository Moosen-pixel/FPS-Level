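; BP_SecurityCamera1 is a stealth security camera that sweeps back and forth and catches the player.
; A self-repeating MoveCamera event alternates between start and end rotations through a FlipFlop, moving the camera mesh with a pause between swings.
; Each Tick, a debug-drawn sphere trace for pawns runs forward from SMLineTrace.
; Hitting the player sets Caught and disables input; the StealthMap reload nodes are never executed.
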(event `self.ReceiveBeginPlay`
  ; Setup
  (`self.MoveCamera`)
  (bind _asbp_first_person_character (cast `/Game/StarterContent/FirstPerson/Blueprints/BP_FirstPersonCharacter` (`GameplayStatics.GetPlayerCharacter` 0)))
  (set `self.BP_FirstPersonCharacter` _asbp_first_person_character))

(event `MoveCamera`
  (bind (_currentrotation_x _currentrotation_y _currentrotation_z) (`KismetMathLibrary.BreakVector` (`self.CurrentRotation`)))
  ; Camera Rotation
  (`/Engine/EditorBlueprintResources/StandardMacros.FlipFlop`
    (:`A`
      (set `self.CurrentRotation` (`self.EndRotation`)))
    (:`B`
      (set `self.CurrentRotation` (`self.StartRotation`))))
  (`KismetSystemLibrary.MoveComponentTo` (`self.SM_SecurityCamera`) (0.0 0.0 0.0) (`KismetMathLibrary.MakeRotator` _currentrotation_x _currentrotation_y _currentrotation_z) false false (`self.Speed`))
  (`KismetSystemLibrary.Delay` (`self.Delay`))
  (`self.MoveCamera`))

(event `self.ReceiveTick`
  (params (DeltaSeconds :type "Float (single-precision)"))
  (`self.Detect`))

(event `Detect`
  (bind _sm_linetrace (`self.SM_LineTrace`))
  (bind _bp_firstpersoncharacter (`self.BP_FirstPersonCharacter`))
  (bind _returnvalue (`SceneComponent.K2_GetComponentLocation` _sm_linetrace))
  ; Linetrace
  (bind _outhit (`KismetSystemLibrary.SphereTraceSingleForObjects` :`Start` _returnvalue :`End` (+ _returnvalue (* (`KismetMathLibrary.GetForwardVector` (`SceneComponent.K2_GetComponentRotation` _sm_linetrace)) (`self.DetectDistance`))) :`Radius` 40.0 :`ObjectTypes` (`|MakeArray` "ObjectTypeQuery3" :!type "EObjectTypeQuery Enum") :`DrawDebugType` "ForOneFrame"))
  (if (== (`.HitActor` (`GameplayStatics.BreakHitResult` _outhit)) _bp_firstpersoncharacter)
    (set `/Game/StarterContent/FirstPerson/Blueprints/BP_FirstPersonCharacter.Caught` true _bp_firstpersoncharacter)
    ; Disable Input, Reset Level
    (`self.DisableInput` (`self.BP_FirstPersonCharacter`) (`GameplayStatics.GetPlayerController` 0))))

(fn `UserConstructionScript`)