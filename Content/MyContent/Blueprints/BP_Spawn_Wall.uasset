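; BP_Spawn_Wall is an actor that shuttles back and forth along a configurable direction, presumably as a moving wall.
; Each Tick adds a world offset of the normalized Direction times Speed, without sweep and without delta-time scaling, so its pace depends on frame rate.
; A looping timer started on BeginPlay negates Direction every MovementDuration seconds to reverse the motion.
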(event `self.ReceiveTick`
  (params (DeltaSeconds :type "Float (single-precision)"))
  ; Wall Movement
  (`self.K2_AddActorWorldOffset` (* (`KismetMathLibrary.Normal` (`self.Direction`)) (`self.Speed`))))

(event `self.ReceiveBeginPlay`
  ; Flip Direction
  (`KismetSystemLibrary.K2_SetTimerDelegate` (delegate `Event_FlipDirection`) (`self.MovementDuration`) true))

(event `Event_FlipDirection`
  ; Flip Direction
  (set `self.Direction` (* (`self.Direction`) -1.0)))

(fn `UserConstructionScript`)