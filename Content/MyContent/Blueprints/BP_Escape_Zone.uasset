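; BP_Escape_Zone is a trigger actor that shows the escape screen when the player enters it.
; On BeginPlay it caches the player's BP_FirstPersonCharacter.
; When that character begins overlapping the Collision component, it enables the mouse cursor and creates and adds Widget_Escape to the viewport.
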(event `self.ReceiveBeginPlay`
  ; Setup
  (bind _asbp_first_person_character (cast `/Game/StarterContent/FirstPerson/Blueprints/BP_FirstPersonCharacter` (`GameplayStatics.GetPlayerCharacter` 0)))
  (set `self.BP_First_Person_Character` _asbp_first_person_character))

(event `self.Collision.OnComponentBeginOverlap`
  (params (OverlappedComponent :type "PrimitiveComponent Object Reference") (OtherActor :type "Actor Object Reference") (OtherComp :type "PrimitiveComponent Object Reference") (OtherBodyIndex :type Integer) (bFromSweep :type Boolean) (SweepResult :type "HitResult Structure (by ref)"))
  (if (== OtherActor (`self.BP_First_Person_Character`))
    (set `PlayerController.bShowMouseCursor` true (`GameplayStatics.GetPlayerController` 0))
    (bind _returnvalue (`|CreateWidget` "/Game/MyContent/UI/Widget_Escape.Widget_Escape_C"))
    (`UserWidget.AddToViewport` _returnvalue 0)))

(fn `UserConstructionScript`)